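; Construction-script actor that lays a chain of instanced static mesh links along an editable spline.
; Each rebuild clears the instanced mesh component, applies the chosen link mesh, and derives spacing and link count from mesh bounds, link scale, an adjust factor and spline length.
; Links follow the spline's position and rotation, with every other one turned 90 degrees to interlock and a roll offset applied.
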(event EventBeginPlay)

(event Collision|EventActorBeginOverlap
  (params (OtherActor :type Actor%20Object%20Reference)))

(event EventTick
  (params (DeltaSeconds :type Float%20%28single-precision%29)))

(fn ConstructionScript
  (CallFunction|ClearInstances (Variables|Default|GetISM_ChainLinks) (Variables|Default|GetLinkMesh) (Variables|Default|GetISM_ChainLinks))
  (bind (_returnvalue _outputpin) (CallFunction|SetInstancesCount (Variables|Default|GetSpline) (Variables|Default|GetISM_ChainLinks) (Variables|Default|GetLinkScale) (Variables|Default|GetAdjust)))
  (for _index (range 0 _returnvalue)
    (CallFunction|BuildLinks (Variables|Default|GetISM_ChainLinks) (Variables|Default|GetLinkScale) _index _index _outputpin (Variables|Default|GetLinkRollOffset))))

(fn ClearInstances
  (params (self2 :type Static%20Mesh%20Component%20Object%20Reference) (NewMesh :type Static%20Mesh%20Object%20Reference) (self3 :type Instanced%20Static%20Mesh%20Component%20Object%20Reference))
  (Components|StaticMesh|SetStaticMesh self2 NewMesh)
  (Components|InstancedStaticMesh|ClearInstances self3))

(fn SetInstancesCount
  (params (Spline :type Spline%20Component%20Object%20Reference) (ISM :type Static%20Mesh%20Component%20Object%20Reference) (LinkScale :type Float%20%28double-precision%29) (Adjust :type Float%20%28double-precision%29))
  (bind _max (Components|StaticMesh|GetLocalBounds ISM))
  (bind _returnvalue (* LinkScale Adjust))
  (bind _returnvalue_2 (* (.x _max) _returnvalue))
  (bind _returnvalue_3 (* (.x _max) 2.0))
  (bind _returnvalue_4 (* _returnvalue_2 -1.0))
  (bind _returnvalue_5 (+ _returnvalue_3 _returnvalue_4))
  (return (- (Math|Float|Truncate (/ (Spline|GetSplineLength Spline) _returnvalue_5)) 1) _returnvalue_5))

(fn BuildLinks
  (params (ISM :type Instanced%20Static%20Mesh%20Component%20Object%20Reference) (LinkScale :type Float%20%28double-precision%29) (Index :type Integer) (Index_b :type Integer) (Count :type Float%20%28double-precision%29) (Roll :type Float%20%28double-precision%29))
  (bind _returnvalue (* Index_b Count))
  (bind _spline (Variables|Default|GetSpline))
  (bind _returnvalue_2 (Spline|GetRotationatDistanceAlongSpline _spline _returnvalue "Local"))
  (Components|InstancedStaticMesh|AddInstance ISM (Math|Transform|MakeTransform (.Location (Math|Transform|BreakTransform (Spline|GetTransformatDistanceAlongSpline _spline _returnvalue "Local" false))) (Math|Rotator|Delta(Rotator) (Math|Rotator|SelectRotator _returnvalue_2 (Math|Rotator|Delta(Rotator) _returnvalue_2 "0.000000,0.000000,90.000000") (== (Math|Integer|%(Integer) Index 2) 1)) (Math|Rotator|MakeRotator Roll 0.0 0.0)) (Math|Conversions|ToVector(Float) LinkScale)) false))